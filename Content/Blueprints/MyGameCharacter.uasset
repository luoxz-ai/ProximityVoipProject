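; Player character Blueprint with camera-relative movement, look with a pitch clamp, hold-to-sprint and a prototype proximity voice chat.
; Every tick it starts networked voice, sets the VOIP sound class volume and sphere-traces around the player for pawns to register or unregister the local talker.
; A hit feeds VoipDistance to set that volume, but its clamped distance falloff math is left unconnected.
; Debug prints and trace drawing remain active.
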(event EventTick
  (params (DeltaSeconds :type Float%20%28single-precision%29))
  ;[1 1 1] Proximity Voip
  (Utilities|FlowControl|Sequence
    (:then_0
      (CallFunction|ProximityVoip))))

(event Input|ActionEvents|InputActionSprint
  (params (Key :type Key%20Structure :default "AnyKey"))
  (bind _charactermovement (Variables|Character|GetCharacterMovement))
  ;[1 1 1] Sprinting
  (:Pressed
    (Variables|/Script/Engine.CharacterMovementComponent|SetMaxWalkSpeed _charactermovement 6e+02))
  (:Released
    (Variables|/Script/Engine.CharacterMovementComponent|SetMaxWalkSpeed _charactermovement 3e+02)))

(event Input|AxisEvents|InputAxisLookRight/Left
  (params (AxisValue :type Float%20%28single-precision%29))
  ;[1 1 1] Look Up/Down, Right/Left
  (Pawn|Input|AddControllerYawInput AxisValue))

(event Input|AxisEvents|InputAxisMoveForward
  (params (AxisValue :type Float%20%28single-precision%29))
  ;[1 1 1] Move Forward, Right
  (Variables|Default|SetMove%20Forward,%20Right%20Active true)
  (Pawn|Input|AddMovementInput (Math|Vector|GetForwardVector (Math|Rotator|MakeRotator 0.0 0.0 (.Yaw (Math|Rotator|BreakRotator (Pawn|GetControlRotation :!class /Script/Engine.Pawn))))) AxisValue false))

(event Input|AxisEvents|InputAxisLookUp/Down
  (params (AxisValue :type Float%20%28single-precision%29))
  (bind _returnvalue (Pawn|GetControlRotation :!class /Script/Engine.Pawn))
  (bind (_roll _pitch _yaw) (Math|Rotator|BreakRotator _returnvalue))
  ;[1 1 1] Look Up/Down, Right/Left
  (Pawn|Input|AddControllerPitchInput AxisValue)
  (Pawn|SetControlRotation (Pawn|GetController) (Math|Rotator|MakeRotator _roll (Math|Float|ClampAngle (+ (* AxisValue 0.1) _pitch) -1.8e+02 3e+01) _yaw)))

(event Input|AxisEvents|InputAxisMoveRight
  (params (AxisValue :type Float%20%28single-precision%29))
  ;[1 1 1] Move Forward, Right
  (Variables|Default|SetMove%20Forward,%20Right%20Active true)
  (Pawn|Input|AddMovementInput (Math|Vector|GetRightVector (Math|Rotator|MakeRotator 0.0 0.0 (.Yaw (Math|Rotator|BreakRotator (Pawn|GetControlRotation :!class /Script/Engine.Pawn))))) AxisValue false))

(fn ConstructionScript)

(fn ProximityVoip
  (bind _returnvalue (Game|Player|GetPlayerPawn 0))
  (bind _returnvalue_2 (Transformation|GetActorLocation _returnvalue))
  (Class|AdvancedVoiceLibrary|StartNetworkedVoice)
  (Class|VictoryBPFunctionLibrary|VictorySoundVolumeChange "/Game/Audio/SoundClassVOIP.SoundClassVoip" (Variables|Default|GetVOIPFloat))
  (Development|PrintString (Utilities|String|ToString(Boolean) (Class|AdvancedVoiceLibrary|IsLocalPlayerTalking)) true true "(R=0.000000,G=0.660000,B=1.000000,A=1.000000)" 2.0)
  (bind (_outhit _returnvalue_3) (Collision|SphereTraceForObjects _returnvalue_2 (+ _returnvalue_2 (Transformation|GetActorUpVector _returnvalue)) 1e+03 (Utilities|Array|MakeArray "ObjectTypeQuery3") true 0 "ForOneFrame"))
  (if _returnvalue_3
    (Class|AdvancedVoiceLibrary|RegisterLocalTalker)
    (Variables|Default|SetVoipFloat (Utilities|VoipDistance (.HitActor (Collision|BreakHitResult _outhit))))
    (Development|PrintString (Utilities|String|ToString(Float) (Variables|Default|GetVoipFloat)) true true "(R=0.000000,G=0.660000,B=1.000000,A=1.000000)" 2.0)
    (else
      (Class|AdvancedVoiceLibrary|UnRegisterLocalTalker)))
  (return))